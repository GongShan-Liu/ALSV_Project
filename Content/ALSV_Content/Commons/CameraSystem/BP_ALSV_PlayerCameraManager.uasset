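; Player camera manager that provides a third-person follow camera for the controlled Character.
; BlueprintUpdateCamera composes an offset behind the pelvis socket with the control rotation, so the view orbits the pelvis.
; The first update places the camera at a fixed offset from the pelvis, and later ones use TInterpTo toward the follow transform.
; A game-time check against zero ends this intro blend by zeroing InterpSpeed, which makes the camera follow without smoothing.
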(fn ConstructionScript)

(fn BlueprintUpdateCamera
  (params (CameraTarget :type Actor%20Object%20Reference))
  ;[0.15 0.15 0.15 0.5 30] # 操纵视觉方案
  ; 1. 相机更新函数是每帧都运行的事件函数
  ; 2. 当前函数的逻辑说明：
  ;     a) 相机的位置以角色的骨骼pelvis的位置减去150(x轴)作为初始位置, 并跟随角色的位移来更新相机的位置
  ;     b) 相机的旋转是以角色的骨骼pelvis为旋转轴心, 并以输入操纵的旋转值来更新相机的旋转视角
  ;     c) 相机运行初期后会有从角色附近位置移动到初始位置的动画, 该动画过程是通过插值节点来更新该相机行为
  (bind _ascharacter (Utilities|Casting|CastToCharacter (Pawn|GetControlledPawn (Game|Player|GetOwningPlayerController))))
  (Utilities|FlowControl|Sequence
    (:then_0
      (if (Variables|Default|Getis_start)
        (Variables|Default|Setis_start false)
        (return (+ (Transformation|GetSocketLocation (Variables|/Script/Engine.Character|GetMesh _ascharacter) (Class|SkinnedMeshComponent|GetSocketBoneName (Variables|/Script/Engine.Character|GetMesh _ascharacter) "pelvis")) "200.000000,500.000000,0.000000") "0, 0, 0" 9e+01 true)))
    (:then_1
      (if (Variables|Default|Getis_start_anim)
        (bind _output_get (Variables|Default|Setis_start_anim (<= (Utilities|Time|GetTimeSeconds) 0.0)))
        (if _output_get
          _
          (else
            (Variables|Default|Setinterp_speed 0.0))))
      (return (.location (Class|KismetMathLibrary|TInterpto (Transformation|GetActorTransform) (Math|Transform|ComposeTransforms (Math|Transform|MakeTransform "-150.000000,0.000000,0.000000") (Math|Transform|MakeTransform (Transformation|GetSocketLocation (Variables|/Script/Engine.Character|GetMesh _ascharacter) (Class|SkinnedMeshComponent|GetSocketBoneName (Variables|/Script/Engine.Character|GetMesh _ascharacter) "pelvis")) (Pawn|GetControlRotation _ascharacter :!class /Script/Engine.Pawn))) (Utilities|Time|GetWorldDeltaSeconds) (Variables|Default|Getinterp_speed))) (.rotation (Class|KismetMathLibrary|TInterpto (Transformation|GetActorTransform) (Math|Transform|ComposeTransforms (Math|Transform|MakeTransform "-150.000000,0.000000,0.000000") (Math|Transform|MakeTransform (Transformation|GetSocketLocation (Variables|/Script/Engine.Character|GetMesh _ascharacter) (Class|SkinnedMeshComponent|GetSocketBoneName (Variables|/Script/Engine.Character|GetMesh _ascharacter) "pelvis")) (Pawn|GetControlRotation _ascharacter :!class /Script/Engine.Pawn))) (Utilities|Time|GetWorldDeltaSeconds) (Variables|Default|Getinterp_speed))) 9e+01 true))))