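; BP_ALSV_Controller is a player controller demonstrating Enhanced Input movement and look for the controlled pawn, labeled as a non-executing example.
; BeginPlay sets IsInput false on the local controller with a valid pawn, so its branch adding IMC_ALSV_Pawn never runs.
; Move and mouse-look actions, also gated by IsInput, would apply control-rotation-relative movement and yaw/pitch input.
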(event Input|EnhancedActionEvents|EnhancedInputActionIA_ALSV_Move
  (params (ActionValue :type Vector%202D%20Structure) (ElapsedSeconds :type Float%20%28double-precision%29) (TriggeredSeconds :type Float%20%28double-precision%29) (InputAction :type Input%20Action%20Object%20Reference :default "/Game/ALSV_Content/Commons/Inputs/Actions/IA_ALSV_Move.IA_ALSV_Move"))
  (bind _returnvalue (Pawn|GetControlRotation :!class /Script/Engine.Controller))
  (bind _returnvalue_2 (Pawn|GetControlledPawn))
  ;[0.15 0.15 0.15 0.5 20] # 操纵输入方案1 (本逻辑不执行, 只作演示)
  ;     使用输入映射的方式来设置输入操作
  ;;[0.15 0.15 0.15 0.5] 输入操作角色的移动
  (if (stale EventBeginPlay _output_get)
    (Pawn|Input|AddMovementInput _returnvalue_2 (Math|Vector|GetRightVector (Math|Rotator|MakeRotator (.roll _returnvalue) 0.0 (.yaw _returnvalue))) (.x ActionValue) false)
    (Pawn|Input|AddMovementInput _returnvalue_2 (Math|Vector|GetForwardVector (Math|Rotator|MakeRotator 0.0 0.0 (.yaw _returnvalue))) (.y ActionValue) false)))

(event Input|EnhancedActionEvents|EnhancedInputActionIA_ALSV_MouseLook
  (params (ActionValue :type Vector%202D%20Structure) (ElapsedSeconds :type Float%20%28double-precision%29) (TriggeredSeconds :type Float%20%28double-precision%29) (InputAction :type Input%20Action%20Object%20Reference :default "/Game/ALSV_Content/Commons/Inputs/Actions/IA_ALSV_MouseLook.IA_ALSV_MouseLook"))
  ;[0.15 0.15 0.15 0.5 20] # 操纵输入方案1 (本逻辑不执行, 只作演示)
  ;     使用输入映射的方式来设置输入操作
  ;;[0.15 0.15 0.15 0.5] 输入操纵的视角控制
  (if (stale EventBeginPlay _output_get)
    (Class|PlayerController|AddYawInput (.x ActionValue))
    (Class|PlayerController|AddPitchInput (.y ActionValue))))

(event EventBeginPlay
  (bind _returnvalue (PlayerController|LocalPlayerSubsystems|GetEnhancedInputLocalPlayerSubsystem))
  (bind (_outfoundpriority _returnvalue_2) (Class|EnhancedInputSubsystemInterface|HasMappingContext _returnvalue "/Game/ALSV_Content/Commons/Inputs/IMC_ALSV_Pawn.IMC_ALSV_Pawn"))
  ;[0.15 0.15 0.15 0.5 20] # 操纵输入方案1 (本逻辑不执行, 只作演示)
  ;     使用输入映射的方式来设置输入操作
  (if (and (Pawn|IsLocalPlayerController) (Utilities|IsValid (Pawn|GetControlledPawn)))
    (bind _output_get (Variables|Default|SetIsInput false))
    (if (and _output_get (not _returnvalue_2))
      (Input|AddMappingContext _returnvalue "/Game/ALSV_Content/Commons/Inputs/IMC_ALSV_Pawn.IMC_ALSV_Pawn" _outfoundpriority "(bIgnoreAllPressedKeysUntilRelease=True,bForceImmediately=False,bNotifyUserSettings=False)")
      (Development|PrintString "input    3"))))

(fn ConstructionScript)