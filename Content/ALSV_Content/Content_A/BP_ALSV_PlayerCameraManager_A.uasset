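; Player camera manager for BP_ALSV_Character_A that overrides BlueprintUpdateCamera to place a boom-style camera behind the character.
; IsFirstPerson selects the nearer of two rear offsets, so neither is a true first-person view.
; TInterpTo blends from that offset toward the stored TestTransform, which is rewritten each update.
; The result is composed with the pelvis bone location and control rotation, with fixed FOV.
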(event EventBeginPlay)

(event Collision|EventActorBeginOverlap
  (params (OtherActor :type Actor%20Object%20Reference)))

(event EventTick
  (params (DeltaSeconds :type Float%20%28single-precision%29)))

(fn ConstructionScript)

(fn BlueprintUpdateCamera
  (params (CameraTarget :type Actor%20Object%20Reference))
  (bind _asbp_alsv_character_a (Utilities|Casting|CastToBP_ALSV_Character_A (Pawn|GetControlledPawn (Game|Player|GetOwningPlayerController))))
  (Variables|Default|Settest_Transform (Class|KismetMathLibrary|TInterpto (Math|Transform|SelectTransform (Math|Transform|MakeTransform "-200.000000,0.000000,0.000000" "0.000000,0.000000,0.000000") (Math|Transform|MakeTransform "-300.000000,0.000000,0.000000" "0.000000,0.000000,0.000000") (Variables|/Game/ALSV_Content/Content_A/BP_ALSV_Character_A.BP_ALSV_Character_A_C|GetIsFirstPerson _asbp_alsv_character_a)) (Variables|Default|Gettest_Transform) (Utilities|Time|GetWorldDeltaSeconds) 58.0))
  (return (.location (Math|Transform|ComposeTransforms (Class|KismetMathLibrary|TInterpto (Math|Transform|SelectTransform (Math|Transform|MakeTransform "-200.000000,0.000000,0.000000" "0.000000,0.000000,0.000000") (Math|Transform|MakeTransform "-300.000000,0.000000,0.000000" "0.000000,0.000000,0.000000") (Variables|/Game/ALSV_Content/Content_A/BP_ALSV_Character_A.BP_ALSV_Character_A_C|GetIsFirstPerson _asbp_alsv_character_a)) (Variables|Default|Gettest_Transform) (Utilities|Time|GetWorldDeltaSeconds) 58.0) (Math|Transform|MakeTransform (Transformation|GetSocketLocation (Variables|/Script/Engine.Character|GetMesh _asbp_alsv_character_a) (Class|SkinnedMeshComponent|GetSocketBoneName (Variables|/Script/Engine.Character|GetMesh _asbp_alsv_character_a) "pelvis")) (Pawn|GetControlRotation _asbp_alsv_character_a :!class /Script/Engine.Pawn)))) (.rotation (Math|Transform|ComposeTransforms (Class|KismetMathLibrary|TInterpto (Math|Transform|SelectTransform (Math|Transform|MakeTransform "-200.000000,0.000000,0.000000" "0.000000,0.000000,0.000000") (Math|Transform|MakeTransform "-300.000000,0.000000,0.000000" "0.000000,0.000000,0.000000") (Variables|/Game/ALSV_Content/Content_A/BP_ALSV_Character_A.BP_ALSV_Character_A_C|GetIsFirstPerson _asbp_alsv_character_a)) (Variables|Default|Gettest_Transform) (Utilities|Time|GetWorldDeltaSeconds) 58.0) (Math|Transform|MakeTransform (Transformation|GetSocketLocation (Variables|/Script/Engine.Character|GetMesh _asbp_alsv_character_a) (Class|SkinnedMeshComponent|GetSocketBoneName (Variables|/Script/Engine.Character|GetMesh _asbp_alsv_character_a) "pelvis")) (Pawn|GetControlRotation _asbp_alsv_character_a :!class /Script/Engine.Pawn)))) 9e+01 true))