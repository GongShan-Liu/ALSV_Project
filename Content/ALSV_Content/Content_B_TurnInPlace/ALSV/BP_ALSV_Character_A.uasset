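; Player character Blueprint for an ALSV turn-in-place setup, handling Enhanced Input movement and mouse look.
; BeginPlay adds the pawn mapping context, move input follows control rotation, and two debug keys switch IsFirstPerson.
; Tick reads the RemainingTurnYaw_aa animation curve but acts on nothing.
; Disconnected experimental nodes would apply that curve as frame-time-scaled actor yaw, with debug prints.
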(event Collision|EventActorBeginOverlap
  (params (OtherActor :type Actor%20Object%20Reference)))

(event EventTick
  (params (DeltaSeconds :type Float%20%28single-precision%29))
  (if (< (Animation|Curves|GetCurveValue (Components|SkeletalMesh|GetAnimInstance (Variables|Character|GetMesh)) "RemainingTurnYaw_aa") -0.001)
    _))

(event Input|EnhancedActionEvents|EnhancedInputActionIA_ALSV_Move
  (params (ActionValue :type Vector%202D%20Structure) (ElapsedSeconds :type Float%20%28double-precision%29) (TriggeredSeconds :type Float%20%28double-precision%29) (InputAction :type Input%20Action%20Object%20Reference :default "/Game/ALSV_Content/Commons/Inputs/Actions/IA_ALSV_Move.IA_ALSV_Move"))
  (bind _returnvalue (Pawn|GetControlRotation :!class /Script/Engine.Pawn))
  (Pawn|Input|AddMovementInput (Math|Vector|GetRightVector (Math|Rotator|MakeRotator (.roll _returnvalue) 0.0 (.yaw _returnvalue))) (.x ActionValue) false)
  (Pawn|Input|AddMovementInput (Math|Vector|GetForwardVector (Math|Rotator|MakeRotator 0.0 0.0 (.yaw _returnvalue))) (.y ActionValue) false))

(event Input|EnhancedActionEvents|EnhancedInputActionIA_ALSV_MouseLook
  (params (ActionValue :type Vector%202D%20Structure) (ElapsedSeconds :type Float%20%28double-precision%29) (TriggeredSeconds :type Float%20%28double-precision%29) (InputAction :type Input%20Action%20Object%20Reference :default "/Game/ALSV_Content/Commons/Inputs/Actions/IA_ALSV_MouseLook.IA_ALSV_MouseLook"))
  (Pawn|Input|AddControllerYawInput (.x ActionValue))
  (Pawn|Input|AddControllerPitchInput (.y ActionValue)))

(event EventBeginPlay
  (bind _returnvalue (PlayerController|LocalPlayerSubsystems|GetEnhancedInputLocalPlayerSubsystem))
  (if (not (.ReturnValue (Class|EnhancedInputSubsystemInterface|HasMappingContext _returnvalue "/Game/ALSV_Content/Commons/Inputs/IMC_ALSV_Pawn.IMC_ALSV_Pawn")))
    (Input|AddMappingContext _returnvalue "/Game/ALSV_Content/Commons/Inputs/IMC_ALSV_Pawn.IMC_ALSV_Pawn" 0 "(bIgnoreAllPressedKeysUntilRelease=True,bForceImmediately=False,bNotifyUserSettings=False)")))

(event Input|KeyboardEvents|DebugKey1
  (params (Key :type Key%20Structure) (ActionValue :type Input%20Action%20Value%20Structure))
  (:Pressed
    (Variables|Default|SetIsFirstPerson true)))

(event Input|KeyboardEvents|DebugKey2
  (params (Key :type Key%20Structure) (ActionValue :type Input%20Action%20Value%20Structure))
  (:Pressed
    (Variables|Default|SetIsFirstPerson false)))

(fn ConstructionScript)