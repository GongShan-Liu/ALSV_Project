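; ALSV character that supports animation-driven turn-in-place, with controller yaw decoupled from the body.
; Tick reads the anim instance's RotationAmount curve and applies it as actor yaw, scaled by delta time against a 30 fps baseline.
; With a single player controller, BeginPlay sets IsInput and adds the Enhanced Input mapping context for camera-relative movement and mouse look.
; Legacy axis events act only while IsInput is false, as an alternative scheme.
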(event EventTick
  (params (DeltaSeconds :type Float%20%28single-precision%29))
  (bind _mesh (Variables|Character|GetMesh))
  (bind _returnvalue (Components|SkeletalMesh|GetAnimInstance _mesh))
  (bind _returnvalue_2 (Animation|Curves|GetCurveValue _returnvalue "RotationAmount"))
  (if (> (Math|Float|Absolute(Float) _returnvalue_2) 0.001)
    (Class|Actor|AddActorWorldRotation (Math|Rotator|MakeRotator 0.0 0.0 (* _returnvalue_2 (/ (Utilities|Time|GetWorldDeltaSeconds) (/ 1.0 3e+01)))))))

(event EventBeginPlay
  (Variables|Default|SetbUseControllerRotationYaw false)
  (CallFunction|InputBeginEvent))

(event Custom|InputBeginEvent
  (bind _returnvalue (Class|GameplayStatics|GetNumPlayerControllers))
  (bind _returnvalue_2 (- _returnvalue 1))
  (bind _returnvalue_3 (Game|GetPlayerController _returnvalue_2))
  (bind _returnvalue_4 (PlayerController|LocalPlayerSubsystems|GetEnhancedInputLocalPlayerSubsystem _returnvalue_3))
  (bind (_outfoundpriority _returnvalue_5) (Class|EnhancedInputSubsystemInterface|HasMappingContext _returnvalue_4 "/Game/ALSV_Content/Commons/Inputs/IMC_ALSV_Pawn.IMC_ALSV_Pawn"))
  ;[0.15 0.15 0.15 0.5 20] # 操纵输入方案1 (项目后续采用该方案)
  ;     使用输入映射的方式来设置输入操作
  (if (== _returnvalue 1)
    (bind _output_get (Variables|Default|SetIsInput true))
    (if (and _output_get (not _returnvalue_5))
      (Input|AddMappingContext _returnvalue_4 "/Game/ALSV_Content/Commons/Inputs/IMC_ALSV_Pawn.IMC_ALSV_Pawn" _outfoundpriority "(bIgnoreAllPressedKeysUntilRelease=True,bForceImmediately=False,bNotifyUserSettings=False)")
      (Development|PrintString "input    1")
      (else
        (Development|PrintString "input    2")))))

(event Input|EnhancedActionEvents|EnhancedInputActionIA_ALSV_Move
  (params (ActionValue :type Vector%202D%20Structure) (ElapsedSeconds :type Float%20%28double-precision%29) (TriggeredSeconds :type Float%20%28double-precision%29) (InputAction :type Input%20Action%20Object%20Reference :default "/Game/ALSV_Content/Commons/Inputs/Actions/IA_ALSV_Move.IA_ALSV_Move"))
  (bind _returnvalue (Pawn|GetControlRotation :!class /Script/Engine.Pawn))
  ;[0.15 0.15 0.15 0.5 20] # 操纵输入方案1 (项目后续采用该方案)
  ;     使用输入映射的方式来设置输入操作
  ;;[0.15 0.15 0.15 0.5] 输入操作角色的移动
  (Pawn|Input|AddMovementInput (Math|Vector|GetRightVector (Math|Rotator|MakeRotator (.roll _returnvalue) 0.0 (.yaw _returnvalue))) (.x ActionValue) false)
  (Pawn|Input|AddMovementInput (Math|Vector|GetForwardVector (Math|Rotator|MakeRotator 0.0 0.0 (.yaw _returnvalue))) (.y ActionValue) false))

(event Input|EnhancedActionEvents|EnhancedInputActionIA_ALSV_MouseLook
  (params (ActionValue :type Vector%202D%20Structure) (ElapsedSeconds :type Float%20%28double-precision%29) (TriggeredSeconds :type Float%20%28double-precision%29) (InputAction :type Input%20Action%20Object%20Reference :default "/Game/ALSV_Content/Commons/Inputs/Actions/IA_ALSV_MouseLook.IA_ALSV_MouseLook"))
  ;[0.15 0.15 0.15 0.5 20] # 操纵输入方案1 (项目后续采用该方案)
  ;     使用输入映射的方式来设置输入操作
  ;;[0.15 0.15 0.15 0.5] 输入操纵的视角控制
  (Pawn|Input|AddControllerYawInput (.x ActionValue))
  (Pawn|Input|AddControllerPitchInput (.y ActionValue)))

(event Input|AxisEvents|InputAxisMoveRight/Left
  (params (AxisValue :type Float%20%28single-precision%29))
  ;[0.15 0.15 0.15 0.5 20] # 操纵输入方案2
  ;     使用项目设置的输入绑定句柄的事件来设置输入操作
  ;;[0.15 0.15 0.15 0.5] 输入操作角色的移动
  (if (not (Variables|Default|GetIsInput))
    (Pawn|Input|AddMovementInput (Transformation|GetActorRightVector (Pawn|GetController)) AxisValue false)))

(event Input|AxisEvents|InputAxisMoveForward/Backward
  (params (AxisValue :type Float%20%28single-precision%29))
  ;[0.15 0.15 0.15 0.5 20] # 操纵输入方案2
  ;     使用项目设置的输入绑定句柄的事件来设置输入操作
  ;;[0.15 0.15 0.15 0.5] 输入操作角色的移动
  (if (not (Variables|Default|GetIsInput))
    (Pawn|Input|AddMovementInput (Transformation|GetActorForwardVector (Pawn|GetController)) AxisValue false)))

(event Input|AxisEvents|InputAxisLookUp/DownMouse
  (params (AxisValue :type Float%20%28single-precision%29))
  ;[0.15 0.15 0.15 0.5 20] # 操纵输入方案2
  ;     使用项目设置的输入绑定句柄的事件来设置输入操作
  ;;[0.15 0.15 0.15 0.5] 输入操纵的视角控制
  (if (not (Variables|Default|GetIsInput))
    (Pawn|Input|AddControllerPitchInput AxisValue)))

(event Input|AxisEvents|InputAxisTurnRight/LeftMouse
  (params (AxisValue :type Float%20%28single-precision%29))
  ;[0.15 0.15 0.15 0.5 20] # 操纵输入方案2
  ;     使用项目设置的输入绑定句柄的事件来设置输入操作
  ;;[0.15 0.15 0.15 0.5] 输入操纵的视角控制
  (if (not (Variables|Default|GetIsInput))
    (Pawn|Input|AddControllerYawInput AxisValue)))

(fn ConstructionScript)